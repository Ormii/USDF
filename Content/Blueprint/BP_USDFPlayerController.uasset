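; Player controller for the USDF game that owns the HUD and end-of-game screens.
; On begin play it creates the HUD widget, then asks the USDF game mode to prepare the stage.
; Stage prepare and end events activate the matching HUD sub-widgets.
; Game over and all-stages-clear add their own widget above the HUD, switch input to UI only and show a centered cursor.
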(event EventBeginPlay
  (bind _returnvalue (UserInterface|CreateWidget (Variables|Default|GetHUDWidgetClass) self))
  (bind _output_get (Variables|Default|SetHUDWidget _returnvalue))
  (UserInterface|Viewport|AddtoViewport _output_get 0)
  (bind _asusdfgame_mode (Utilities|Casting|CastToUSDFGameMode (Game|GetGameMode)))
  (Class|USDFGameMode|PrepareGameStage _asusdfgame_mode))

(event EventTick
  (params (DeltaSeconds :type Float%20%28single-precision%29)))

(event EventOnGameOver
  (bind (_sizex _sizey) (HUD|GetViewportSize))
  (bind _returnvalue (UserInterface|CreateWidget "/Game/Blueprint/Widget/BP_USDFGameOverWidget.BP_USDFGameOverWidget_C" self))
  (UserInterface|Viewport|AddtoViewport _returnvalue 1)
  (Input|SetInputModeUIOnly self _returnvalue "DoNotLock" true)
  (Variables|Default|SetbShowMouseCursor true)
  (Class|PlayerController|SetMouseLocation (/ _sizex 2) (/ _sizey 2)))

(event EventOnAllGameStageClear
  (bind (_sizex _sizey) (HUD|GetViewportSize))
  (bind _returnvalue (UserInterface|CreateWidget "/Game/Blueprint/Widget/WBP_USDFAllStageClearWidget.WBP_USDFAllStageClearWidget_C" self))
  (UserInterface|Viewport|AddtoViewport _returnvalue 1)
  (Input|SetInputModeUIOnly self 0 "DoNotLock" true)
  (Variables|Default|SetbShowMouseCursor true)
  (Class|PlayerController|SetMouseLocation (/ _sizex 2) (/ _sizey 2)))

(event EventOnPrepareGameStage
  (Class|USDFPrepareStageWidget|OnActivatePrepareStage (Variables|/Script/USDF.USDFPlayerHUDWidget|GetPrepareStageWidget (Variables|Default|GetHUDWidget))))

(event EventOnEndGameStage
  (Class|USDFEndStageWidget|OnActivateEndStage (Variables|/Script/USDF.USDFPlayerHUDWidget|GetEndStageWidget (Variables|Default|GetHUDWidget))))

(fn ConstructionScript)