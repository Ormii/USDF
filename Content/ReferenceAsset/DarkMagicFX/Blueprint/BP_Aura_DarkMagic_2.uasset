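; BP_Aura_DarkMagic_2 is a dark magic aura effect actor that applies an overlay material to an animated skeletal mesh.
; The construction script creates a dynamic instance of the overlay material, assigns it to the mesh's overlay slot, and feeds in the base color and dissolve opacity range from variables.
; On BeginPlay it enables input for the first player controller and plays the Ability_E animation on a loop.
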(event EventBeginPlay
  (Input|EnableInput (Game|GetPlayerController 0))
  (Components|Animation|PlayAnimation (Variables|Default|GetSkeletalMesh) "/Game/ReferenceAsset/DarkMagicFX/Demo/Ability_E.Ability_E" true))

(fn ConstructionScript
  (bind _returnvalue (Rendering|Material|CreateDynamicMaterialInstance (Variables|Default|GetOverlayMaterial) "None" "None" :!class /Script/Engine.KismetMaterialLibrary))
  (bind _output_get (Variables|Default|SetoverlaymDynamic _returnvalue))
  (Rendering|Material|SetOverlayMaterial (Variables|Default|GetSkeletalMesh) _output_get :!class /Script/Engine.MeshComponent)
  ;[1 1 1] base color
  (Rendering|Material|SetVectorParameterValue (Variables|Default|GetoverlaymDynamic) "Base_Color" (Variables|Controller|GetBase_Color) :!class /Script/Engine.MaterialInstanceDynamic)
  ;[1 1 1] Dissolve Range
  (Rendering|Material|SetScalarParameterValue (Variables|Default|GetoverlaymDynamic) "Opacity_Min" (Variables|Default|GetOpacity_Min) :!class /Script/Engine.MaterialInstanceDynamic)
  (Rendering|Material|SetScalarParameterValue (Variables|Default|GetoverlaymDynamic) "Opacity_Max" (Variables|Default|GetOpacity_Max) :!class /Script/Engine.MaterialInstanceDynamic))