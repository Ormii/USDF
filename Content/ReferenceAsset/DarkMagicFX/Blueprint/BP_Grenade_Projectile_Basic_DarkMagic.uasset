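; Dark magic grenade projectile that explodes once it has used up its Health through physics hits.
; Each hit on Sphere1 decrements Health; at zero or below, it stops the Niagara effect and disables the sphere's physics, collision and visibility.
; It spawns a Niagara explosion at the hit location, then destroys the actor after a short delay.
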(event OnComponentHit(Sphere1)
  (params (HitComponent :type Primitive%20Component%20Object%20Reference) (OtherActor :type Actor%20Object%20Reference) (OtherComp :type Primitive%20Component%20Object%20Reference) (NormalImpulse :type Vector :default "0, 0, 0") (Hit :type Hit%20Result%20Structure%20%28by%20ref%29))
  (bind _sphere1 (Variables|Default|GetSphere1))
  (bind _output_get (Variables|Default|Sethealth (- (Variables|Default|Gethealth) 1)))
  (Math|Integer|CompareInt 0 _output_get
    (:>
      _)
    (:==
      _))
  (Utilities|FlowControl|Sequence
    (:then_0
      (Components|Activation|Deactivate (Variables|Default|GetNiagara))
      (Physics|SetSimulatePhysics _sphere1 false)
      (Collision|SetCollisionEnabled _sphere1 "NoCollision")
      (Rendering|SetVisibility _sphere1 false false)
      (Utilities|FlowControl|Delay 4.0)
      (Actor|DestroyActor))
    (:then_1
      (Niagara|SpawnSystematLocation "/Game/ReferenceAsset/DarkMagicFX/Niagara/Projectile/NS_Explosion_Grenade_DarkMagic.NS_Explosion_Grenade_DarkMagic" (.Location (Collision|BreakHitResult Hit)) (Transformation|GetActorRotation))
      (Utilities|FlowControl|Delay 3.0)
      (Actor|DestroyActor))))

(fn ConstructionScript)