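; BP_Shooting_Small_DarkMagic is an effect emitter actor that repeatedly fires small dark magic projectiles, apparently for showcasing the DarkMagicFX pack.
; After a random startup delay on BeginPlay, it spawns ProjectileBP at one-tenth scale, randomly offset in X and Z from its location and oriented along its Arrow component.
; The NextArrow event then calls itself after a random delay of one to two seconds, forming an endless firing loop.
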(event Custom|NextArrow
  (bind _returnvalue (Math|Random|RandomFloatinRange -1e+02 1e+02))
  (Game|SpawnActorfromClass (Variables|Default|GetProjectileBP) (Math|Transform|MakeTransform (+ (Transformation|GetActorLocation) (Math|Vector|MakeVector _returnvalue 0.0 _returnvalue)) (.rotation (Transformation|GetWorldTransform (Variables|Default|GetArrow))) "0.100000,0.100000,0.100000") "Undefined" "SelectDefaultAtRuntime" 0 0)
  (Utilities|FlowControl|Delay (Math|Random|RandomFloatinRange 1.0 2.0))
  (CallFunction|NextArrow))

(event EventBeginPlay
  (bind _returnvalue (Math|Random|RandomFloatinRange -1e+02 1e+02))
  (Utilities|FlowControl|Delay (Math|Random|RandomFloat))
  (Game|SpawnActorfromClass (Variables|Default|GetProjectileBP) (Math|Transform|MakeTransform (+ (Transformation|GetActorLocation) (Math|Vector|MakeVector _returnvalue 0.0 _returnvalue)) (.rotation (Transformation|GetWorldTransform (Variables|Default|GetArrow))) "0.100000,0.100000,0.100000") "Undefined" "SelectDefaultAtRuntime" 0 0)
  (Utilities|FlowControl|Delay (Math|Random|RandomFloatinRange 1.0 2.0))
  (CallFunction|NextArrow))

(fn ConstructionScript)