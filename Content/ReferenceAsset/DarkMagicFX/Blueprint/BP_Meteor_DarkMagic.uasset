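; BP_Meteor_DarkMagic is a spawner that repeatedly opens a dark magic meteor portal effect and launches a projectile from it.
; After a startup delay, it spawns the Niagara portal at its location, facing along its Arrow component, then spawns the ProjectileBP class at reduced scale with the same orientation.
; A fixed pause, written as a random range with equal bounds, precedes NextArrow, which loops the sequence indefinitely.
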(event Custom|NextArrow
  (bind _returnvalue (Transformation|GetActorLocation))
  (bind _arrow (Variables|Default|GetArrow))
  (bind _returnvalue_2 (Transformation|GetWorldTransform _arrow))
  (Niagara|SpawnSystematLocation "/Game/ReferenceAsset/DarkMagicFX/Niagara/Meteor/NS_Portal_Meteor_DarkMagic.NS_Portal_Meteor_DarkMagic" _returnvalue (.rotation _returnvalue_2))
  (Utilities|FlowControl|Delay 1.0)
  (Game|SpawnActorfromClass (Variables|Default|GetProjectileBP) (Math|Transform|MakeTransform _returnvalue (.rotation _returnvalue_2) "0.100000,0.100000,0.100000") "Undefined" "SelectDefaultAtRuntime" 0 0)
  (Utilities|FlowControl|Delay (Math|Random|RandomFloatinRange 3.0 3.0))
  (CallFunction|NextArrow))

(event EventBeginPlay
  (bind _returnvalue (Transformation|GetActorLocation))
  (bind _arrow (Variables|Default|GetArrow))
  (bind _returnvalue_2 (Transformation|GetWorldTransform _arrow))
  (Utilities|FlowControl|Delay 1.0)
  (Niagara|SpawnSystematLocation "/Game/ReferenceAsset/DarkMagicFX/Niagara/Meteor/NS_Portal_Meteor_DarkMagic.NS_Portal_Meteor_DarkMagic" _returnvalue (.rotation _returnvalue_2))
  (Utilities|FlowControl|Delay 1.0)
  (Game|SpawnActorfromClass (Variables|Default|GetProjectileBP) (Math|Transform|MakeTransform _returnvalue (.rotation _returnvalue_2) "0.100000,0.100000,0.100000") "Undefined" "SelectDefaultAtRuntime" 0 0)
  (Utilities|FlowControl|Delay (Math|Random|RandomFloatinRange 3.0 3.0))
  (CallFunction|NextArrow))

(fn ConstructionScript)